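; Player character Blueprint that handles camera zoom and owns the player's on-screen UI.
; The zoom axis input adjusts the CameraBoom arm length within a clamped range.
; BeginPlay creates WBP_PlayerUI and adds it to the viewport, and OnUpdateScore forwards new scores to that widget.
; A TODO notes that the spring arm and camera are still to be added to C++.
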(event EventBeginPlay
  (bind _returnvalue (UserInterface|CreateWidget "/Game/Core/Blueprints/UI/WBP_PlayerUI.WBP_PlayerUI_C"))
  (bind _output_get (Variables|Default|SetMainUI _returnvalue))
  (UserInterface|Viewport|AddtoViewport _output_get 0))

(event EventOnUpdateScore
  (params (newScore :type Integer))
  (Default|UpdateScore (Variables|Default|GetMainUI) newScore))

(event Input|AxisEvents|InputAxisIAx_Zoom
  (params (AxisValue :type Float%20%28single-precision%29))
  (bind _cameraboom (Variables|Default|GetCameraBoom))
  ;[0.9792 0 0] Zoom Input - TODO add Springarm/Camera to C++
  (Variables|/Script/Engine.SpringArmComponent|SetTargetArmLength _cameraboom (Math|Float|Clamp(Float) (+ (* AxisValue 2e+01) (Variables|/Script/Engine.SpringArmComponent|GetTargetArmLength _cameraboom)) 3e+02 1e+03)))

(fn ConstructionScript)